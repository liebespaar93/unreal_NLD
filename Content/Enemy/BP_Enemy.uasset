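; BP_Enemy is an AI enemy character that chases and attacks the player and offers randomized loot on death.
; A repeating AIMoveTo triggers a montage attack that fires an end dispatcher, while helpers attach a KA47, expose a patrol route and set walk speed by state.
; Hits update health, and death fills the interaction widget with items rolled from an enum at a decreasing chance.
; SheathGun is an unfinished stub.
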(event Custom|ChasePlayer
  ;[1 1 1] 어느정도 이동후 사격 준비자세 만들것
  (AI|AIMoveTo self "0, 0, 0" (Game|GetPlayerCharacter 0) 5.0 false
    (:OnSuccess
      (CallFunction|Attack)
      (Utilities|FlowControl|Delay 2.2)
      (CallFunction|ChasePlayer))))

(event Custom|Attack
  (Animation|Montage|PlayMontage (Variables|Character|GetMesh) "/Game/Animation/tossgrenade_UE_Montage.tossgrenade_UE_Montage"
    (:OnCompleted
      _)
    (:OnInterrupted
      _))
  ;[1 1 1] 실행이 완료되었을때 와  실행이 실패 하였을때 끝을 넨다
  (Default|CallOnAttackEnd))

(event Custom|WeaponFire
  ;[1 1 1] 무기 들기
  (bind _returnvalue (Game|SpawnActorfromClass "/Game/Enemy/Weapons/BP_KA47.BP_KA47_C" (Transformation|GetActorTransform) "Undefined" "MultiplyWithRoot" 0 0))
  (Transformation|AttachComponentToComponent _returnvalue (Variables|Character|GetMesh) "hand_r_weapon_socket" "SnapToTarget" "SnapToTarget" "SnapToTarget" true)
  (Variables|Default|SetIsWeaponEquip true))

(event Custom|EnemyDead
  ;[1 1 1] 죽은 후 로직
  (bind _itemlist (CallFunction|CreateItemList))
  (bind _aswg_interaction_wiget (Utilities|Casting|CastToWG_InteractionWiget (UserInterface|GetWidget (Variables|Default|GetWidget))))
  (Default|SetDropItems _aswg_interaction_wiget _itemlist))

(event Custom|EnemyHit
  (params (Damage :type Float%20%28double-precision%29))
  ;[1 1 1] 데미지 받는 로직
  (bind _output_get (Variables|Default|SetHealth (- Damage (Variables|Default|GetHealth))))
  (if (< _output_get 0.0)
    (CallFunction|EnemyDead)
    (Development|PrintString "Enemy Hit")))

(event Custom|ItemRemove
  (params (Item :type S%20Item%20Structure))
  (bind _items (Variables|Default|GetItems))
  ;[1 1 1] Item 삭제
  (Utilities|Array|RemoveIndex _items (Utilities|Array|FindItem _items Item))
  (Development|PrintString "Item delete in enemy  "))

(event Custom|SheathGun
  (bind _notifyname (Animation|Montage|PlayMontage (Variables|Character|GetMesh) 0)
    (:OnNotifyBegin
      (switch name _notifyname))))

(event Custom|EnemyItemsVisible
  (params (visible :type ESlateVisibility%20Enum :default "Visible"))
  ;[1 1 1] 죽은 후 로직
  (Widget|SetVisibility (UserInterface|GetWidget (Variables|Default|GetWidget)) visible))

(event EventBeginPlay
  (Utilities|FlowControl|Sequence
    (:then_0
      (CallFunction|EnemyItemsVisible "Hidden"))))

(fn ConstructionScript)

(fn CreateItemList
  (Utilities|FlowControl|Sequence
    (:then_0
      (Variables|Default|SetItemSpawn 0.9)
      (while (< (Math|Random|RandomFloat) (Variables|Default|GetItemSpawn))
        (Variables|Default|SetItemSpawn (- (Variables|Default|GetItemSpawn) 0.1))
        (Variables|Default|SetItemIndex (Math|Random|RandomIntegerinRange 1 13))
        (Variables|Default|Seti 0)
        (bind _enumvalue (|ForEachE_Item)
          (:LoopBody
            (Variables|Default|Seti (+ (Variables|Default|Geti) 1))
            (if (== (Variables|Default|Geti) (Variables|Default|GetItemIndex))
              (Utilities|Array|Add (Variables|Default|GetItems) (Utilities|Struct|MakeS_Item (Utilities|String|EnumtoString _enumvalue) "test info")))))))
    (:then_1
      (return (Variables|Default|GetItems)))))

(fn GetPatrolRoute
  (return (Variables|Default|GetPatrolRoute)))

(fn SetMovementSpeed
  (params (SpeedState :type E_MovementSpeed%20Enum :default "NewEnumerator0"))
  (bind _output_get (Variables|/Script/Engine.CharacterMovementComponent|SetMaxWalkSpeed (Variables|Character|GetCharacterMovement) (Utilities|Select :Index SpeedState :NewEnumerator0 0.0 :NewEnumerator1 1e+02 :NewEnumerator2 3e+02 :NewEnumerator3 5e+01 :NewEnumerator4 3e+01)))
  (return _output_get))