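; BP_DoorSingle is a single swinging door actor that can start open or be omitted entirely.
; BeginPlay offsets the yaw if IsOpen, then uses HaveDoor to set visibility and mesh collision.
; OpenDoor, CloseDoor and ToggleDoor set IsOpen, which Tick reads to step CurrRotation toward MaxRotation or zero at Speed.
; CloseDoor also zeroes the rotation immediately, though Tick then reapplies the decreasing CurrRotation.
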(event Custom|OpenDoor
  ;[1 1 1] Open Door
  (Variables|Default|SetIsOpen true))

(event Custom|CloseDoor
  ;[1 1 1] Close Door
  (Transformation|SetRelativeRotation (Variables|Default|GetDoor) "0, 0, 0" false false)
  (Variables|Default|SetIsOpen false))

(event Custom|ToggleDoor
  ;[1 1 1] Test for
  (if (Variables|Default|GetIsOpen)
    (CallFunction|CloseDoor)
    (else
      (CallFunction|OpenDoor))))

(event EventBeginPlay
  (bind _door (Variables|Default|GetDoor))
  (bind _doormesh (Variables|Default|GetDoorMesh))
  (bind _havedoor (Variables|Default|GetHaveDoor))
  (Utilities|FlowControl|Sequence
    (:then_0
      ;[1 1 1] Open
      (if (Variables|Default|GetIsOpen)
        (Transformation|SetRelativeRotation _door (Math|Rotator|Delta(Rotator) (Variables|/Script/Engine.SceneComponent|GetRelativeRotation _door) "0.000000,90.000000,0.000000") false false)))
    (:then_1
      ;[1 1 1] Check Have Door
      (Rendering|SetVisibility (Variables|Default|GetDoor) _havedoor true)
      (if _havedoor
        (Collision|SetCollisionEnabled _doormesh "QueryAndPhysics")
        (else
          (Collision|SetCollisionEnabled _doormesh "NoCollision"))))))

(event Collision|EventActorBeginOverlap
  (params (OtherActor :type Actor%20Object%20Reference)))

(event EventTick
  (params (DeltaSeconds :type Float%20%28single-precision%29))
  (if (Variables|Default|GetIsOpen)
    ;[1 1 1] 회전 열림
    (if (< (Variables|Default|GetCurrRotation) (Variables|Default|GetMaxRotation))
      (bind _output_get (Variables|Default|SetCurrRotation (+ (Variables|Default|GetCurrRotation) (* DeltaSeconds (Variables|Default|GetSpeed)))))
      (Transformation|SetRelativeRotation (Variables|Default|GetDoor) (Math|Rotator|MakeRotator 0.0 0.0 _output_get) false false))
    (else
      ;[1 1 1] Comment
      (if (>= (Variables|Default|GetCurrRotation) 0.0)
        (bind _output_get_2 (Variables|Default|SetCurrRotation (- (Variables|Default|GetCurrRotation) (* DeltaSeconds (Variables|Default|GetSpeed)))))
        (Transformation|SetRelativeRotation (Variables|Default|GetDoor) (Math|Rotator|MakeRotator 0.0 0.0 _output_get_2) false false)))))

(fn ConstructionScript)