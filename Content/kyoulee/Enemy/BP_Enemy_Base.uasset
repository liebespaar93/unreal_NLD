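; Base enemy character that fights with a rifle, heals, grants XP and becomes lootable on death.
; AI-facing events play equip, fire and heal montages, act on their notifies and signal completion through dispatchers.
; Gunfire is randomized one-to-three-shot bursts of line traces with weighted spread.
; Hits reduce health, drive physical-animation reactions and track per-bone HP, with lethal headshots and empty limb-shot hooks; death generates random loot for the interaction widget.
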(event Custom|GunEquip
  ;[1 1 1] Take The Bullet
  ;;[1 1 1] Comment
  (bind _notifyname (Animation|Montage|PlayMontage (Variables|Character|GetMesh) "/Game/kyoulee/Animations/Montage/RiflePullOut_UE_Montage.RiflePullOut_UE_Montage")
    (:OnCompleted
      (Default|CallOnGunEquiped))
    (:OnNotifyBegin
      ;;[1 1 1] notice 을확인하여 반응
      (switch name _notifyname
        (:HoldGun
          ;;[1 1 1] Create Weapon to Enemy position
          (bind _returnvalue (Game|SpawnActorfromClass "/Game/kyoulee/Weapon/BP_KA47.BP_KA47_C" (Transformation|GetActorTransform) "Undefined" "MultiplyWithRoot" 0 0))
          ;;[1 1 1] Setting Enemy State of TakeGun
          (Variables|Default|SetIsTakeWeapon true)
          ;;[1 1 1] Make Actor to Enemy Component
          ;; Join Enemy Mesh with Socket name
          ;; and  set target of U want
          ;; after setting setting all rules to snap to target
          (bind _output_get (Variables|Default|SetWeaponActor _returnvalue))
          (Transformation|AttachComponentToComponent _output_get (Variables|Character|GetMesh) "hand_r_Weapon_Socket" "SnapToTarget" "SnapToTarget" "SnapToTarget" true))))))

(event Custom|FireTarget
  ;[1 1 1] 총쏘기
  (CallFunction|FireGun)
  (Utilities|FlowControl|Delay 0.4)
  (if (Math|Random|RandomBool)
    (CallFunction|FireGun)
    (Utilities|FlowControl|Delay 0.4)
    (if (Math|Random|RandomBool)
      (CallFunction|FireGun)
      (Utilities|FlowControl|Delay 0.4)))
  ;;[1 1 1] 새로히 even dis patcher 를 만들어 준다
  (Default|CallOnAttackEnd))

(event Custom|HealDecrease
  (params (Damage :type Float%20%28double-precision%29))
  ;[1 1 1] Damage Enemy funtion
  (bind _output_get (Variables|State|SetHealth (Math|Float|Clamp(Float) (- (Variables|State|GetHealth) Damage) 0.0 (Variables|State|GetMaxHealth))))
  (if (<= _output_get 0.0)
    (if (not (Variables|State|GetIsDead))
      (Variables|State|SetIsDead true)
      (CallFunction|EnemyDead)
      (bind _asbp_third_person_character (Utilities|Casting|CastToBP_ThirdPersonCharacter (Game|Player|GetPlayerPawn 0)))
      (Default|AddExp _asbp_third_person_character (Variables|Default|GetXP)))))

(event Custom|GunEnquip
  ;[1 1 1] Destroy equip gun
  ;;[1 1 1] play carry the gun aninimation of enemy
  (bind _notifyname (Animation|Montage|PlayMontage (Variables|Character|GetMesh) "/Game/kyoulee/Animations/Montage/RiflePutAway_UE_Montage.RiflePutAway_UE_Montage")
    (:OnCompleted
      ;;[1 1 1] make wait for animation is done
      (Default|CallOnGUnUnequiped))
    (:OnNotifyBegin
      ;;[1 1 1] notice애니메이션 활용
      (switch name _notifyname
        (:ReleaseGun
          ;;[1 1 1] destory gun actor
          (Actor|DestroyActor (Variables|Default|GetWeaponActor))
          ;;[1 1 1] SET Gun no gun in hand
          (Variables|Default|SetIsTakeWeapon false))))))

(event Custom|FireGun
  (bind _weaponactor (Variables|Default|GetWeaponActor))
  (bind _returnvalue (Transformation|GetActorLocation _weaponactor))
  ;[1 1 1] 총쏘기
  (bind _notifyname (Animation|Montage|PlayMontage (Variables|Character|GetMesh) "/Game/kyoulee/Animations/Montage/FiringRifle_Idle__UE_Montage.FiringRifle_Idle__UE_Montage")
    (:OnNotifyBegin
      (switch name _notifyname
        (:Fire
          ;;[1 1 1] 총에서 적에게 레이 추적
          (bind _asaic_enemy_base (Utilities|Casting|CastToAIC_Enemy_base (AI|GetAIController self)))
          (bind _attacktarget (Variables|/Game/kyoulee/Enemy/AI/AIC_Enemy_base.AIC_Enemy_base_C|GetAttackTarget _asaic_enemy_base)
            (:then
              (bind _newpoint (CallFunction|MultRandomFov (Transformation|GetActorLocation _attacktarget) _returnvalue 8e+01))
              (bind (_outhit _returnvalue_2) (Collision|LineTraceByChannel _returnvalue _newpoint "TraceTypeQuery1" false 0 "ForDuration"))
              (if _returnvalue_2
                (bind _asbp_third_person_character (Utilities|Casting|CastToBP_ThirdPersonCharacter (.HitActor (Collision|BreakHitResult _outhit))))
                (Default|GetDamaged _asbp_third_person_character (Variables|State|GetDamage))))
            (:else)))))))

(event Custom|EnemyDead
  ;[1 1 1] 죽은 후 로직
  (bind _asaic_enemy_base (Utilities|Casting|CastToAIC_Enemy_base (AI|GetAIController self)))
  (Default|SetStateasDead _asaic_enemy_base)
  (AI|ClearFocus _asaic_enemy_base)
  (bind _items (CallFunction|CreateItemList))
  (Variables|Default|SetItems _items)
  (Default|DeadReaction (Variables|Default|GetBP_physicalAnimationComp))
  (bind _returnvalue (Audio|CreateSound2D "/Game/kyoulee/Sounds/Assets/SD_HitOWWW.SD_HitOWWW" 1.0 1.0 0.0 0))
  (Audio|Components|Audio|Play _returnvalue 2.0))

(event Custom|HitAction
  (params (Hit :type Hit%20Result%20Structure%20%28by%20ref%29) (BaseDamage :type Float%20%28single-precision%29))
  (bind (_bblockinghit _binitialoverlap _time _distance _location _impactpoint _normal _impactnormal _physmat _hitactor _hitcomponent _hitbonename _bonename _hititem _elementindex _faceindex _tracestart) (Collision|BreakHitResult Hit))
  (bind _bodypiecehp (Variables|HpState|GetBodyPieceHp))
  (bind _returnvalue (- _tracestart _location))
  (bind _returnvalue_2 (Math|Vector|Normalize _returnvalue 1.0))
  ;[1 1 1] 외부 맞는 함수 호출
  (CallFunction|HealDecrease BaseDamage)
  (Default|HitReaction (Variables|Default|GetBP_physicalAnimationComp) Hit (Variables|State|GetIsDead))
  (Utilities|FlowControl|Sequence
    (:then_0
      ;;[1 1 1] 피 이펙트 만들기
      (Effects|SpawnEmitteratLocation "/Game/Realistic_Starter_VFX_Pack_Vol2/Particles/Blood/P_Blood_Splat_Cone.P_Blood_Splat_Cone" _location (Math|Rotator|MakeRotator 0.0 9e+01 (Class|KismetMathLibrary|DegAtan2 (.y _returnvalue_2) (.x _returnvalue_2))))
      (if (not (Variables|State|GetIsDead))
        (bind _returnvalue_3 (Audio|CreateSound2D "/Game/kyoulee/Sounds/SC_Hurt.SC_Hurt" 1.0 1.0 0.0 0))
        (Audio|Components|Audio|Play _returnvalue_3 0.0)))
    (:then_1
      ;;[1 1 1] Cut body
      (CallFunction|MakeHpState)
      (bind _enemyhpstate (CallFunction|GetEnemyBoneEnum _hitbonename))
      ;;;[1 1 1] 왜 배열이 안채워질까?
      (if (<= (- (Utilities|Array|Get(acopy) (Variables|HpState|GetBodyPieceHp) (Utilities|Select :Index _enemyhpstate :NewEnumerator4 0 :NewEnumerator5 1 :NewEnumerator3 2 :NewEnumerator2 3 :NewEnumerator0 4 :NewEnumerator1 5)) BaseDamage) 0.0)
        (Utilities|Array|SetArrayElem _bodypiecehp (Utilities|Select :Index _enemyhpstate :NewEnumerator4 0 :NewEnumerator5 1 :NewEnumerator3 2 :NewEnumerator2 3 :NewEnumerator0 4 :NewEnumerator1 5) 0.0)
        (switch int (Utilities|Select :Index _enemyhpstate :NewEnumerator4 0 :NewEnumerator5 1 :NewEnumerator3 2 :NewEnumerator2 3 :NewEnumerator0 4 :NewEnumerator1 5)
          (:0
            (Utilities|FlowControl|DoOnce false
              (:Completed
                (CallFunction|HealDecrease 9999.0)
                (CallFunction|HeadShot))))
          (:2
            (CallFunction|ArmLeftShot))
          (:3
            (CallFunction|ArmRightShot))
          (:4
            (CallFunction|LegLeftShot))
          (:5
            (CallFunction|LegRightShot)))
        (else
          (Utilities|Array|SetArrayElem _bodypiecehp (Utilities|Select :Index _enemyhpstate :NewEnumerator4 0 :NewEnumerator5 1 :NewEnumerator3 2 :NewEnumerator2 3 :NewEnumerator0 4 :NewEnumerator1 5) (- (Utilities|Array|Get(acopy) (Variables|HpState|GetBodyPieceHp) (Utilities|Select :Index _enemyhpstate :NewEnumerator4 0 :NewEnumerator5 1 :NewEnumerator3 2 :NewEnumerator2 3 :NewEnumerator0 4 :NewEnumerator1 5)) BaseDamage)))))))

(event Custom|ItemRemove
  (params (Item :type F%20Slot%20Struct%20Structure))
  (bind _items (Variables|Default|GetItems))
  ;[1 1 1] Item 삭제
  (Utilities|Array|RemoveIndex _items (Utilities|Array|FindItem _items Item))
  (Development|PrintString "Item delete in enemy  "))

(event Custom|Healing
  (params (heal :type Float%20%28double-precision%29))
  ;[1 1 1] Comment
  (bind _notifyname (Animation|Montage|PlayMontage (Variables|Character|GetMesh) "/Game/kyoulee/Animations/Montage/HealSelf_UE_Montage.HealSelf_UE_Montage")
    (:OnCompleted
      (Default|CallOnHealingEnd))
    (:OnNotifyBegin
      ;;[1 1 1] 반으로 나누어 힐
      (switch name _notifyname
        (:Heal
          (Variables|State|SetHealth (Math|Float|Clamp(Float) (+ (/ (Variables|State|GetHealth) 2.0) heal) 0.0 (Variables|State|GetMaxHealth))))))))

(event Custom|PopItem
  (params (index :type Integer) (player :type Actor%20Object%20Reference))
  (bind _items (Variables|Default|GetItems))
  (bind _output (Utilities|Array|Get(acopy) _items index))
  ;[1 1 1] Pop item
  (if (> (Utilities|Array|Length (Variables|Default|GetItems)) 0)
    (bind _asbp_third_person_character (Utilities|Casting|CastToBP_ThirdPersonCharacter player))
    (Default|AddtoInventory (Variables|/Game/ThirdPerson/Blueprints/BP_ThirdPersonCharacter.BP_ThirdPersonCharacter_C|GetInventory%20System _asbp_third_person_character) (Utilities|String|StringToName (.ItemID (Utilities|Struct|BreakFSlotStruct _output))) 1)
    (CallFunction|ItemRemove _output)))

(event EventBeginPlay
  (Utilities|FlowControl|Sequence
    (:then_0
      ;[1 1 1] 체력 정하기
      (Variables|State|SetHealth (Variables|State|GetMaxHealth)))
    (:then_1
      ;[1 1 1] Get ai controler
      (bind _asaic_enemy_base (Utilities|Casting|CastToAIC_Enemy_base (AI|GetAIController self)))
      (Variables|Default|SetAs%20AIC%20Enemy%20Base _asaic_enemy_base))))

(event EventUnEquipWeapon
  ;[1 1 1] 인터페이스 작업 모음
  (CallFunction|GunEnquip))

(event EventEquipWeapon
  ;[1 1 1] 인터페이스 작업 모음
  (CallFunction|GunEquip))

(event EventAttack
  ;[1 1 1] 인터페이스 작업 모음
  (CallFunction|FireTarget))

(event Game|Damage|EventAnyDamage
  (params (Damage :type Float%20%28single-precision%29) (DamageType :type Damage%20Type%20Object%20Reference) (InstigatedBy :type Controller%20Object%20Reference) (DamageCauser :type Actor%20Object%20Reference))
  ;[1 1 1] Damage Enemy funtion
  (bind _output_get (Variables|State|SetHealth (Math|Float|Clamp(Float) (- (Variables|State|GetHealth) (stale Custom|HealDecrease Damage)) 0.0 (Variables|State|GetMaxHealth))))
  (if (<= _output_get 0.0)
    (if (not (Variables|State|GetIsDead))
      (Variables|State|SetIsDead true)
      (CallFunction|EnemyDead)
      (bind _asbp_third_person_character (Utilities|Casting|CastToBP_ThirdPersonCharacter (Game|Player|GetPlayerPawn 0)))
      (Default|AddExp _asbp_third_person_character (Variables|Default|GetXP)))))

(event EventHeal
  (params (Heal :type Float%20%28double-precision%29))
  ;[1 1 1] 인터페이스 작업 모음
  (CallFunction|Healing Heal))

(fn ConstructionScript)

(fn MultRandomFov
  (params (TargetPoint :type Vector) (StartPoint :type Vector) (Fov :type Float%20%28double-precision%29))
  (bind _returnvalue (/ Fov 2.0))
  (bind _value (CallFunction|GaussianDist 0.7))
  (bind _value_2 (CallFunction|GaussianDist 0.7))
  (return (+ (Class|KismetMathLibrary|QuatRotateVector (Math|Conversions|ToQuaternion(Rotator) (Math|Rotator|MakeRotator (* _value _returnvalue) 0.0 (* _value_2 _returnvalue))) (- TargetPoint StartPoint)) StartPoint)))

(fn GaussianDist
  (params (weight :type Float%20%28double-precision%29))
  ;[1 1 1] 확율 모양 만들기
  (Variables|Default|SetGaussianValue (Math|Random|RandomFloatinRange 0.0 1.0))
  (Variables|Default|SetGaussianDistribution 0.0)
  (while (> (Variables|Default|GetGaussianValue) weight)
    (Variables|Default|SetGaussianDistribution (+ (Variables|Default|GetGaussianDistribution) 0.1))
    (Variables|Default|SetGaussianValue (Math|Random|RandomFloatinRange 0.0 1.0)))
  ;[1 1 1] 쁠마
  (bind _output_get (Variables|Default|SetGaussianValue (Math|Random|RandomFloatinRange 0.0 1.0)))
  (return (* (Variables|Default|GetGaussianDistribution) (- (> _output_get 0.5) 0.5) 2.0)))

(fn CreateItemList
  (Utilities|FlowControl|Sequence
    (:then_0
      (Variables|Default|SetItem%20Spawn 0.9)
      (while (< (Math|Random|RandomFloatinRange 0.0 1.0) (Variables|Default|GetItem%20Spawn))
        (Variables|Default|SetItem%20Spawn (- (Variables|Default|GetItem%20Spawn) 0.1))
        (Variables|Default|SetItem%20Index (Math|Random|RandomIntegerinRange 1 13))
        (Variables|Default|SetI 0)
        (bind _enumvalue (|ForEachE_Item)
          (:LoopBody
            (Variables|Default|SetI (+ (Variables|Default|GetI) 1))
            (if (== (Variables|Default|GetI) (Variables|Default|GetItem%20Index))
              (Utilities|Array|Add (Variables|Default|GetItems) (Utilities|Struct|MakeFSlotStruct (Utilities|String|EnumtoString _enumvalue) 1)))))))
    (:then_1
      (return (Variables|Default|GetItems)))))

(fn LineTarcingEvent
  (params (OwnerPlayer :type Actor%20Object%20Reference))
  (Utilities|Casting|CastToBP_ThirdPersonCharacter OwnerPlayer)
  (if (Variables|State|GetIsDead)
    (Utilities|IsValid (LocalVariables|GetWidget_valid)
      (:Is%20Not%20Valid
        (bind _returnvalue (UserInterface|CreateWidget "/Game/kyoulee/Interaction/Item/WG_InteractionWiget.WG_InteractionWiget_C"))
        (LocalVariables|SetWidget_valid _returnvalue)
        (Default|SetDropItems _returnvalue (Variables|Default|GetItems))
        (UserInterface|Viewport|AddtoViewport _returnvalue 0)
        (bind _widget_valid (LocalVariables|GetWidget_valid)
          (:then
            (return _widget_valid true))
          (:else
            (return _widget_valid false)))))))

(fn GetEnemyBoneEnum
  (params (BoneName :type Name))
  ;[1 1 1] 아,. array로 만들걸
  (if (== BoneName "head")
    (Variables|HpState|SetEnumEnemyHpIndex 0)
    (return (Utilities|Select :Index (Variables|HpState|GetEnumEnemyHpIndex) :Option%200 "NewEnumerator4" :Option%201 "NewEnumerator5" :Option%202 "NewEnumerator3" :Option%203 "NewEnumerator2" :Option%204 "NewEnumerator0" :Option%205 "NewEnumerator1"))
    (elif (== BoneName "spine_05")
      (Variables|HpState|SetEnumEnemyHpIndex 1)
      (return (Utilities|Select :Index (Variables|HpState|GetEnumEnemyHpIndex) :Option%200 "NewEnumerator4" :Option%201 "NewEnumerator5" :Option%202 "NewEnumerator3" :Option%203 "NewEnumerator2" :Option%204 "NewEnumerator0" :Option%205 "NewEnumerator1"))
      (elif (== BoneName "upperarm_l")
        (Variables|HpState|SetEnumEnemyHpIndex 2)
        (return (Utilities|Select :Index (Variables|HpState|GetEnumEnemyHpIndex) :Option%200 "NewEnumerator4" :Option%201 "NewEnumerator5" :Option%202 "NewEnumerator3" :Option%203 "NewEnumerator2" :Option%204 "NewEnumerator0" :Option%205 "NewEnumerator1"))
        (elif (== BoneName "upperarm_r")
          (Variables|HpState|SetEnumEnemyHpIndex 3)
          (return (Utilities|Select :Index (Variables|HpState|GetEnumEnemyHpIndex) :Option%200 "NewEnumerator4" :Option%201 "NewEnumerator5" :Option%202 "NewEnumerator3" :Option%203 "NewEnumerator2" :Option%204 "NewEnumerator0" :Option%205 "NewEnumerator1"))
          (elif (== BoneName "thigh_l")
            (Variables|HpState|SetEnumEnemyHpIndex 4)
            (return (Utilities|Select :Index (Variables|HpState|GetEnumEnemyHpIndex) :Option%200 "NewEnumerator4" :Option%201 "NewEnumerator5" :Option%202 "NewEnumerator3" :Option%203 "NewEnumerator2" :Option%204 "NewEnumerator0" :Option%205 "NewEnumerator1"))
            (elif (== BoneName "thigh_r")
              (Variables|HpState|SetEnumEnemyHpIndex 5)
              (return (Utilities|Select :Index (Variables|HpState|GetEnumEnemyHpIndex) :Option%200 "NewEnumerator4" :Option%201 "NewEnumerator5" :Option%202 "NewEnumerator3" :Option%203 "NewEnumerator2" :Option%204 "NewEnumerator0" :Option%205 "NewEnumerator1")))))))))

(fn MakeHpState
  (bind _bodypiecehp (Variables|HpState|GetBodyPieceHp))
  (Utilities|Array|Add _bodypiecehp (Variables|HpState|GetHpHead))
  (Utilities|Array|Add _bodypiecehp (Variables|HpState|GetHpBody))
  (Utilities|Array|Add _bodypiecehp (Variables|HpState|GetHpArm_L))
  (Utilities|Array|Add _bodypiecehp (Variables|HpState|GetHpArm_R))
  (Utilities|Array|Add _bodypiecehp (Variables|HpState|GetHpLeg_L))
  (Utilities|Array|Add _bodypiecehp (Variables|HpState|GetHpLeg_R))
  (return _bodypiecehp))

(fn HeadShot)

(fn ArmLeftShot)

(fn ArmRightShot)

(fn LegLeftShot)

(fn LegRightShot)

(fn GetCurrentHealth
  (return (Variables|State|GetHealth)))

(fn GetCurrentMaxHealth
  (return (Variables|State|GetMaxHealth)))

(fn GetIdleRange
  ;[1 1 1] 어텍 거리와 서성이는 거리를 정한다
  (return (Variables|AI|GetAttack%20Radius) (Variables|AI|GetDefend%20Radius)))

(fn GetPatrolRoute
  (return (Variables|AI|GetPatrolRoute)))

(fn IIsDead
  (return (Variables|State|GetIsDead)))

(fn SetMovementSpeed
  (params (Speed :type E_MovementSpeed%20Enum :default "NewEnumerator0"))
  ;[1 1 1] Set Character Movement max speed
  (bind _output_get (Variables|/Script/Engine.CharacterMovementComponent|SetMaxWalkSpeed (Variables|Character|GetCharacterMovement) (Utilities|Select :Index Speed :NewEnumerator0 0.0 :NewEnumerator1 1.5e+02 :NewEnumerator2 3e+02 :NewEnumerator3 6e+02)))
  (return _output_get))