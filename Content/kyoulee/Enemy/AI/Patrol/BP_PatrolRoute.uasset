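; BP_PatrolRoute is a patrol path for enemy AI, defined by the points of a spline.
; IncrementPatrolRoute steps the current index along the spline and flips direction at the first and last points, so patrols ping-pong along the route.
; GetSplinePointAsWorldPosition returns the current point's world location along with the route's movement speed.
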(event Custom|IncrementPatrolRoute
  ;[1 1 1] Make Patrol
  ;;[1 1 1] Control Patrol index
  (bind _output_get (Variables|Default|SetPatrolIndex (+ (Variables|Default|GetPatrolIndex) (Variables|Default|GetDirection))))
  ;;[1 1 1] increase index setting when over then spline count
  (if (>= _output_get (- (Spline|GetNumberOfSplinePoints (Variables|Default|GetPatrolRoute)) 1))
    (Variables|Default|SetDirection -1)
    (else
      ;;[1 1 1] decrease index setting when low then 0
      (if (<= (Variables|Default|GetPatrolIndex) 0)
        (Variables|Default|SetDirection 1)))))

(fn ConstructionScript)

(fn GetSplinePointasWorldPosition
  ;[1 1 1] return world Location of spline now index
  (return (Spline|GetLocationatSplinePoint (Variables|Default|GetPatrolRoute) (Variables|Default|GetPatrolIndex) "World") (Variables|Keys|GetMovementSpeed)))